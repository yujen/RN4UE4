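; SignalAllRPC is a Blueprint that signals a named RPC to all RakNet servers when a configurable key is pressed.
; Tick polls the first player controller for the key press and calls the RakNet signal-all-servers function with the RPC identifier.
; An optional debug flag prints the identifier to confirm the call.
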(event EventBeginPlay)

(event EventTick
  (params (DeltaSeconds :type Float%20%28single-precision%29))
  (bind _rpc_signal_identifier (Variables|Default|GetRPC%20Signal%20Identifier))
  (if (Game|Player|WasInputKeyJustPressed (Game|GetPlayerController 0) (Variables|Default|GetKeyToPress))
    (Class|RakNetRP|RPrpcSignalAllServers (Variables|Default|GetRakNet) _rpc_signal_identifier)
    (if (Variables|Default|GetDisplayCall)
      (Development|PrintString (Utilities|String|Append _rpc_signal_identifier " Called")))))